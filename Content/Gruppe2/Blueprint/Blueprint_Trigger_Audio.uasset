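; A one-shot audio trigger actor that plays a dialogue line as the first-person player character passes it.
; Until it has played, Tick checks whether the player is within TriggerRadius, scaled by 100, then a dot product against the actor's forward vector confirms they are on its front side.
; It then sets HasPlayed, waits a configurable delay and plays the Dialogue at the world origin with a debug print.
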(event `self.ReceiveTick`
  (params (DeltaSeconds :type "Float (single-precision)"))
  (if (not (`self.HasPlayed`))
    (bind _asbp_first_person_character (cast `/Game/StoryAdvTemplate/Blueprints/BP_FirstPersonCharacter` (`GameplayStatics.GetPlayerCharacter` 0)))
    (if (< (`KismetMathLibrary.Vector_Distance` (`SceneComponent.K2_GetComponentLocation` (`Actor.RootComponent` _asbp_first_person_character)) (`self.K2_GetActorLocation`)) (* (`self.Trigger Radius`) 100.0))
      (`self.Check_hasPassed`))))

(event `PlayDialogue`
  (set `self.HasPlayed` true)
  (`KismetSystemLibrary.Delay` (`self.Delay`))
  (`GameplayStatics.PlayDialogueAtLocation` (`self.Dialogue`) (`self.Context`) (0.0 0.0 0.0) (struct) 1.0 1.0 0.0 null)
  (`KismetSystemLibrary.PrintString` "Playing Sound")
  (`KismetSystemLibrary.Delay` 2.0))

(event `Check_hasPassed`
  (bind _asbp_first_person_character (cast `/Game/StoryAdvTemplate/Blueprints/BP_FirstPersonCharacter` (`GameplayStatics.GetPlayerCharacter` 0)))
  (if (> (`KismetMathLibrary.Dot_VectorVector` (`KismetMathLibrary.Normal` (- (`SceneComponent.K2_GetComponentLocation` (`Actor.RootComponent` _asbp_first_person_character)) (`self.K2_GetActorLocation`))) (`SceneComponent.GetForwardVector` (`self.RootComponent`))) 0.0)
    (`self.PlayDialogue`)))

(fn `UserConstructionScript`)