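; Actor component for a keycard-controlled machine that slides its owning actor open like a door when the player comes near.
; Once Unlock_Machine sets the unlocked flag, a Tick check triggers opening when the first-person character is within a fixed radius.
; While opening, Tick offsets the owner along its forward vector by SlideSpeed each frame, without delta-time scaling.
; A delay of SlideDistance over SlideSpeed stops the slide and clears the unlock.
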(event `self.ReceiveBeginPlay`)

(event `self.ReceiveTick`
  (params (DeltaSeconds :type "Float (single-precision)"))
  (bind _returnvalue (`self.GetOwner`))
  (`self.IsInDistance`)
  (if (`self.IsOpening`)
    (`Actor.K2_AddActorWorldOffset` _returnvalue (* (`Actor.GetActorForwardVector` _returnvalue) (`self.slideSpeed`)) false false)))

(event `Unlock_Machine`
  (`KismetSystemLibrary.PrintString` "The machine is unlocked." true true (struct :`G` 0.66 :`B` 1.0 :`A` 1.0) 1.0)
  (set `self.isUnlocked` true))

(event `Open_Machine`
  (if (`self.isUnlocked`)
    (`KismetSystemLibrary.Delay` 0.0)
    (set `self.IsOpening` true)
    (`KismetSystemLibrary.Delay` (/ (`self.slideDistance`) (`self.slideSpeed`)))
    (set `self.IsOpening` false)
    (set `self.isUnlocked` false)))

(event `IsInDistance`
  (if (`self.IsOpening`)
    _
    (elif (`self.isUnlocked`)
      (bind _asbp_first_person_character (cast `/Game/StoryAdvTemplate/Blueprints/BP_FirstPersonCharacter` (`GameplayStatics.GetPlayerCharacter` 0)))
      (if (< (`KismetMathLibrary.Vector_Distance` (`SceneComponent.K2_GetComponentLocation` (`Actor.RootComponent` _asbp_first_person_character)) (`Actor.K2_GetActorLocation` (`self.GetOwner`))) 200.0)
        (`KismetSystemLibrary.PrintString` "Opening the door")
        (`self.Open_Machine`)))))