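; Footsteps Blueprint, likely an actor component, that plays step sounds as player character 0 moves.
; Each tick it measures the distance moved since the previous tick and drains a cooldown scaled by that against an assumed walking speed, so faster movement means quicker steps.
; When the cooldown drops below zero, it resets and plays a random 2D sound from cupboard, door and drawer opening assets.
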(event `self.ReceiveTick`
  (params (DeltaSeconds :type "Float (single-precision)"))
  (set `self.Delta Seconds` DeltaSeconds)
  (set `self.CurrentLocation` (`Actor.K2_GetActorLocation` (`GameplayStatics.GetPlayerCharacter` 0)))
  (set `self.PlayerSpeed` (`KismetMathLibrary.VSize` (- (`self.CurrentLocation`) (`self.PreviousLocation`))))
  (bind _output_get (set `self.StepCooldown` (- (`self.StepCooldown`) (* (`self.Delta Seconds`) (/ (`self.PlayerSpeed`) (`self.AssumedWalkingSpeed`))))))
  (set `self.PreviousLocation` (`self.CurrentLocation`))
  (if (> 0.0 _output_get)
    (set `self.StepCooldown` (`self.StepFrequency`))
    (`GameplayStatics.SpawnSound2D` (`KismetArrayLibrary.Array_Random` (`|MakeArray` "/Game/StoryAdvTemplate/Sound/Waves/S_Open_Cupboard_01.S_Open_Cupboard_01" "/Game/StoryAdvTemplate/Sound/Waves/S_Open_Door_01.S_Open_Door_01" "/Game/StoryAdvTemplate/Sound/Waves/S_Open_Drawer_01.S_Open_Drawer_01" :!type "SoundWave Object Reference")) 1.0 1.0 0.0 null)))