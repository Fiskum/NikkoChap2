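; Actor component for a keycard duck that detects when the player finds the keycard by looking at it from a specific angle.
; Each tick it checks that the first-person camera is close and its forward vector closely matches the owner's up vector via a dot product.
; If alignment still holds after a one-second delay, it unlocks the referenced vending machine's sliding-object component, prints a found message and hides a nested child component.
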(event `self.ReceiveBeginPlay`)

(event `self.ReceiveTick`
  (params (DeltaSeconds :type "Float (single-precision)"))
  (bind _returnvalue (`self.GetOwner`))
  (bind _asbp_first_person_character (cast `/Game/StoryAdvTemplate/Blueprints/BP_FirstPersonCharacter` (`GameplayStatics.GetPlayerCharacter` 0)))
  (bind _camera (`/Game/StoryAdvTemplate/Blueprints/BP_FirstPersonCharacter.Camera` _asbp_first_person_character))
  (if (> 50.0 (`KismetMathLibrary.Vector_Distance` (`SceneComponent.K2_GetComponentLocation` _camera) (`Actor.K2_GetActorLocation` _returnvalue)))
    (bind _returnvalue_2 (> (`KismetMathLibrary.Dot_VectorVector` (`SceneComponent.GetForwardVector` _camera) (`Actor.GetActorUpVector` _returnvalue)) 0.9))
    (if _returnvalue_2
      (`KismetSystemLibrary.Delay` 1.0)
      (if _returnvalue_2
        (set `/Game/Gruppe2/Blueprint/Blueprint_AC_SlidingObject.isLocked` false (`Actor.GetComponentByClass` (`self.Vending Machine`) "/Game/Gruppe2/Blueprint/Blueprint_AC_SlidingObject.Blueprint_AC_SlidingObject_C"))
        (`KismetSystemLibrary.PrintString` "Keycard has been found!")
        (`SceneComponent.SetVisibility` (`SceneComponent.GetChildComponent` (`SceneComponent.GetChildComponent` (`Actor.RootComponent` (`self.GetOwner`)) 0) 0) false false)))))