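; Actor component that slides its owner along a direction when the player gazes at it from nearby, with optional locking after use.
; Tick checks a 200-unit range and compares camera forward to the owner root's first child via dot product, rechecking after 0.75 seconds before sliding and calling the empty OnActivate event.
; Sliding adds an unswept, frame-rate-dependent offset each tick until a distance-over-speed delay ends it.
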(event `On Activate`)

(event `self.ReceiveTick`
  (params (DeltaSeconds :type "Float (single-precision)"))
  (`self.Slide`)
  (`self.CheckRange`)
  (`self.CheckButton`))

(event `Slide`
  (if (`self.isSliding`)
    (`Actor.K2_AddActorWorldOffset` (`self.GetOwner`) (* (`self.Direction`) (`self.slideSpeed`)) false false)
    (`KismetSystemLibrary.Delay` (/ (`self.slideDistance`) (`self.slideSpeed`)))
    (set `self.isSliding` false)
    (if (`self.lockAfterUse`)
      (set `self.isLocked` true))))

(event `CheckRange`
  (set `self.isInRange` (> 200.0 (`KismetMathLibrary.Vector_Distance` (`SceneComponent.K2_GetComponentLocation` (`Character.Mesh` (`GameplayStatics.GetPlayerCharacter` 0))) (`Actor.K2_GetActorLocation` (`self.GetOwner`))))))

(event `CheckButton`
  (if (`self.isInRange`)
    (if (not (`self.isSliding`))
      (bind _asbp_first_person_character (cast `/Game/StoryAdvTemplate/Blueprints/BP_FirstPersonCharacter` (`GameplayStatics.GetPlayerCharacter` 0)))
      (bind _camera (`/Game/StoryAdvTemplate/Blueprints/BP_FirstPersonCharacter.Camera` _asbp_first_person_character))
      (bind _returnvalue (> (`KismetMathLibrary.Dot_VectorVector` (`SceneComponent.GetForwardVector` _camera) (`KismetMathLibrary.Normal` (- (`SceneComponent.K2_GetComponentLocation` (`SceneComponent.GetChildComponent` (`Actor.RootComponent` (`self.GetOwner`)) 0)) (`SceneComponent.K2_GetComponentLocation` _camera)))) (`self.ButtonCone`)))
      (if _returnvalue
        (`KismetSystemLibrary.Delay` 0.75)
        (if _returnvalue
          (if (not (`self.isLocked`))
            (set `self.isSliding` true)
            (`self.On Activate`)))))))